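; Pistol pickup Blueprint that lets the player take the weapon and holster it on the character.
; On the Interaction input, it casts the first player character to Player and calls its pickup message.
; It then snaps the pistol to the PistolRengaine socket on the player mesh, hides the widget, destroys the sphere and turns off custom depth rendering.
; The graph itself contains no overlap or range check.
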(event `InputAction|Interaction`
  (params (Key :type "Key Structure"))
  (:`Pressed`
    (bind _asplayer (cast `/Game/002-BluePrints/Player/Player` (`GameplayStatics.GetPlayerCharacter` 0)))
    (message `/Game/002-BluePrints/Armes/PickUpInteraction.PickUpPistol` _asplayer)
    (`self.K2_AttachToComponent` self (`Character.Mesh` _asplayer) "PistolRengaine" "SnapToTarget" "SnapToTarget" "SnapToTarget" true)
    (`SceneComponent.SetVisibility` (`self.Widget`) false false)
    (`ActorComponent.K2_DestroyComponent` (`self.Sphere`))
    (`PrimitiveComponent.SetRenderCustomDepth` (`self.StaticMesh`) false)))

(fn `UserConstructionScript`
  (`parent.UserConstructionScript`))